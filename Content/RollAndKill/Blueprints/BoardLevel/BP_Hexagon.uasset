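; BP_Hexagon is a board-level actor that tracks whose turn it is and positions the dice for that player.
; SetPlayerTurn cycles the PlayerTurn enum through four values, then moves the Dice component to the matching relative location in PlayerTurnDiceLocations.
; BeginPlay triggers this once, so the initial turn value advances immediately.
; The dice color function is an empty stub.
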(event `self.ReceiveBeginPlay`
  (`self.Set Player Turn`))

(event `Set Player Turn`
  (`self.SelectNextPlayer`)
  (`self.SetDiceLocationBasedOnThePlayerEnum` (`KismetMathLibrary.Conv_ByteToInt` (`self.PlayerTurn`))))

(fn `SelectNextPlayer`
  (switch `/Game/RollAndKill/Blueprints/BoardLevel/Enums/PlayerTurnEnum` (`self.PlayerTurn`)
    (:`NewEnumerator0`
      (set `self.PlayerTurn` "NewEnumerator1"))
    (:`NewEnumerator1`
      (set `self.PlayerTurn` "NewEnumerator2"))
    (:`NewEnumerator2`
      (set `self.PlayerTurn` "NewEnumerator3"))
    (:`NewEnumerator3`
      (set `self.PlayerTurn` "NewEnumerator0"))))

(fn `SetDiceColorBasedOnThePlayerEnum`
  (params (PlayerTurn :type "/Game/RollAndKill/Blueprints/BoardLevel/Enums/PlayerTurnEnum Enum" :default "NewEnumerator0")))

(fn `SetDiceLocationBasedOnThePlayerEnum`
  (params (NextPlayer :type Integer))
  (`SceneComponent.K2_SetRelativeLocation` (`self.Dice`) (`|GetArrayItem` (`self.PlayerTurnDiceLocations`) NextPlayer) false false))

(fn `UserConstructionScript`)