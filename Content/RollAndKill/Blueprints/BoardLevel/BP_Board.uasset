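; BP_Board runs a four-player, Ludo-style board with turn cycling, four pawns per colour and a dice repositioned each turn.
; It binds to BP_Dice's roll event and has per-colour functions that swap pawn materials and bind or unbind click events.
; Moving a clicked pawn adds the roll to its stored index, teleports it to that point on its colour's spline, clears highlights and advances the turn.
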(event `self.ReceiveBeginPlay`
  (`self.Set Player Turn`))

(event `Set Player Turn`
  (`self.SelectNextPlayer`)
  (`self.SetDiceLocationBasedOnThePlayerEnum`))

(event `Move Pawn`
  (params (TouchedComponent :type "PrimitiveComponent Object Reference") (ButtonPressed :type "Key Structure" :default "None"))
  (`SceneComponent.K2_SetWorldLocation` TouchedComponent (`self.GettingLocationForThePawnToMove` TouchedComponent) false false)
  (`self.UnHighlightAndRemoveOnClickEvents`)
  (`self.Set Player Turn`)
  (`/Game/RollAndKill/Blueprints/BoardLevel/BP_Dice.RotaionComplete` (`self.DiceRef`)))

(event `UnHighlightAndRemoveOnClickEvents`
  (`self.HighlightAndMakeMovableRed` true)
  (`self.HighlightAndMakeMovableGreen` true)
  (`self.HighlightAndMakeMovableBlue` true)
  (`self.HighlightAndMakeMovableYellow` true))

(fn `GetCurrentPlayerSplinePath`
  (returns (Spline :type "SplineComponent Object Reference"))
  (locals (SplinePath :type "SplineComponent Object Reference"))
  (switch `/Game/RollAndKill/Blueprints/BoardLevel/Enums/PlayerTurnEnum` (`self.PlayerTurn`)
    (:`NewEnumerator0`
      (set `local.SplinePath` (`self.RedPath`)))
    (:`NewEnumerator1`
      (set `local.SplinePath` (`self.GreenPath`)))
    (:`NewEnumerator2`
      (set `local.SplinePath` (`self.BluePath`)))
    (:`NewEnumerator3`
      (set `local.SplinePath` (`self.YellowPath`))))
  (return (`local.SplinePath`)))

(fn `GetPlayerCurrentSelectedPawnLocation`
  (params (TouchedPawn :type "PrimitiveComponent Object Reference"))
  (returns (Index :type Integer))
  (locals (CurrentTouchedPawnIndex :type Integer))
  (switch `string` (`KismetSystemLibrary.GetObjectName` TouchedPawn)
    (:`PR1`
      (set `local.CurrentTouchedPawnIndex` 0 :!label _label))
    (:`PR2`
      (set `local.CurrentTouchedPawnIndex` 1 :!label _label_2))
    (:`PR3`
      (set `local.CurrentTouchedPawnIndex` 2 :!label _label_3))
    (:`PR4`
      (set `local.CurrentTouchedPawnIndex` 3 :!label _label_4))
    (:`PG1`
      (goto _label))
    (:`PG2`
      (goto _label_2))
    (:`PG3`
      (goto _label_3))
    (:`PG4`
      (goto _label_4))
    (:`PB1`
      (goto _label))
    (:`PB2`
      (goto _label_2))
    (:`PB3`
      (goto _label_3))
    (:`PB4`
      (goto _label_4))
    (:`PY1`
      (goto _label))
    (:`PY2`
      (goto _label_2))
    (:`PY3`
      (goto _label_3))
    (:`PY4`
      (goto _label_4)))
  (return (`local.CurrentTouchedPawnIndex`)))

(fn `GetPlayersCurrentPawnLocationArray`
  (returns (Array :type "Array of Integer"))
  (locals (CurrentPlayersPawnLocationArray :type "Array of Integer"))
  (return))

(fn `GettingLocationForThePawnToMove`
  (params (TouchedPawn :type "PrimitiveComponent Object Reference"))
  (returns (ReturnValue :type "Vector Structure"))
  (locals (MoveIndex :type Integer))
  (bind _output (`|GetArrayItem` (select `/Game/RollAndKill/Blueprints/BoardLevel/Enums/PlayerTurnEnum` (`self.PlayerTurn`) :`NewEnumerator0` (`self.RedPawnLocations`) :`NewEnumerator1` (`self.GreenPawnLocations`) :`NewEnumerator2` (`self.BluePawnLocations`) :`NewEnumerator3` (`self.YellowPawnLocations`)) (`self.GetPlayerCurrentSelectedPawnLocation` TouchedPawn)))
  (bind _output_get (set `local.MoveIndex` (+ _output (`/Game/RollAndKill/Blueprints/BoardLevel/BP_Dice.RandomDiceSelectedNumber` (`self.DiceRef`)))))
  (`|VariableSetRef` _output _output_get)
  (bind _result (`/Engine/EditorBlueprintResources/StandardMacros.DecrementInt` (`local.MoveIndex`))
    (:`  `
      (return (`SplineComponent.GetLocationAtSplinePoint` (`self.GetCurrentPlayerSplinePath`) _result "World")))))

(fn `HighlightAndMakeMovableBlue`
  (params (IsUnhighlight :type Boolean))
  (bind _pb2 (`self.PB2`))
  (bind _pb2_2 (`self.PB2`))
  (if IsUnhighlight
    (`PrimitiveComponent.SetMaterial` _pb2 0 "/Engine/VREditor/BasicMeshes/MI_Cube_02.MI_Cube_02")
    (`PrimitiveComponent.SetMaterial` (`self.PB4`) 0 "/Engine/VREditor/BasicMeshes/MI_Cube_02.MI_Cube_02")
    (`PrimitiveComponent.SetMaterial` (`self.PB1`) 0 "/Engine/VREditor/BasicMeshes/MI_Cube_02.MI_Cube_02")
    (`PrimitiveComponent.SetMaterial` (`self.PB3`) 0 "/Engine/VREditor/BasicMeshes/MI_Cube_02.MI_Cube_02")
    (clear `PrimitiveComponent.OnClicked` _pb2)
    (clear `PrimitiveComponent.OnClicked` (`self.PB4`))
    (clear `PrimitiveComponent.OnClicked` (`self.PB1`))
    (clear `PrimitiveComponent.OnClicked` (`self.PB3`))
    (else
      (`PrimitiveComponent.SetMaterial` _pb2_2 0 "/Engine/MapTemplates/Sky/M_BlackBackground.M_BlackBackground")
      (`PrimitiveComponent.SetMaterial` (`self.PB4`) 0 "/Engine/MapTemplates/Sky/M_BlackBackground.M_BlackBackground")
      (`PrimitiveComponent.SetMaterial` (`self.PB1`) 0 "/Engine/MapTemplates/Sky/M_BlackBackground.M_BlackBackground")
      (`PrimitiveComponent.SetMaterial` (`self.PB3`) 0 "/Engine/MapTemplates/Sky/M_BlackBackground.M_BlackBackground")
      (add `PrimitiveComponent.OnClicked` _pb2_2 (`|CreateDelegate` :!event `Move Pawn`))
      (add `PrimitiveComponent.OnClicked` (`self.PB4`) (`|CreateDelegate` :!event `Move Pawn`))
      (add `PrimitiveComponent.OnClicked` (`self.PB1`) (`|CreateDelegate` :!event `Move Pawn`))
      (add `PrimitiveComponent.OnClicked` (`self.PB3`) (`|CreateDelegate` :!event `Move Pawn`)))))

(fn `HighlightAndMakeMovableGreen`
  (params (IsUnhighlight :type Boolean))
  (bind _pg1 (`self.PG1`))
  (bind _pg1_2 (`self.PG1`))
  (if IsUnhighlight
    (`PrimitiveComponent.SetMaterial` _pg1_2 0 "/Engine/VREditor/BasicMeshes/MI_Cube_04.MI_Cube_04")
    (`PrimitiveComponent.SetMaterial` (`self.PG4`) 0 "/Engine/VREditor/BasicMeshes/MI_Cube_04.MI_Cube_04")
    (`PrimitiveComponent.SetMaterial` (`self.PG3`) 0 "/Engine/VREditor/BasicMeshes/MI_Cube_04.MI_Cube_04")
    (`PrimitiveComponent.SetMaterial` (`self.PG2`) 0 "/Engine/VREditor/BasicMeshes/MI_Cube_04.MI_Cube_04")
    (clear `PrimitiveComponent.OnClicked` _pg1_2)
    (clear `PrimitiveComponent.OnClicked` (`self.PG4`))
    (clear `PrimitiveComponent.OnClicked` (`self.PG3`))
    (clear `PrimitiveComponent.OnClicked` (`self.PG2`))
    (else
      (`PrimitiveComponent.SetMaterial` _pg1 0 "/Engine/MapTemplates/Sky/M_BlackBackground.M_BlackBackground")
      (`PrimitiveComponent.SetMaterial` (`self.PG4`) 0 "/Engine/MapTemplates/Sky/M_BlackBackground.M_BlackBackground")
      (`PrimitiveComponent.SetMaterial` (`self.PG3`) 0 "/Engine/MapTemplates/Sky/M_BlackBackground.M_BlackBackground")
      (`PrimitiveComponent.SetMaterial` (`self.PG2`) 0 "/Engine/MapTemplates/Sky/M_BlackBackground.M_BlackBackground")
      (add `PrimitiveComponent.OnClicked` _pg1 (`|CreateDelegate` :!event `Move Pawn`))
      (add `PrimitiveComponent.OnClicked` (`self.PG4`) (`|CreateDelegate` :!event `Move Pawn`))
      (add `PrimitiveComponent.OnClicked` (`self.PG3`) (`|CreateDelegate` :!event `Move Pawn`))
      (add `PrimitiveComponent.OnClicked` (`self.PG2`) (`|CreateDelegate` :!event `Move Pawn`)))))

(fn `HighlightAndMakeMovableRed`
  (params (IsUnhighlight :type Boolean))
  (bind _pr4 (`self.PR4`))
  (if IsUnhighlight
    (`PrimitiveComponent.SetMaterial` _pr4 0 "/Engine/VREditor/BasicMeshes/MI_Cube_03.MI_Cube_03")
    (`PrimitiveComponent.SetMaterial` (`self.PR3`) 0 "/Engine/VREditor/BasicMeshes/MI_Cube_03.MI_Cube_03")
    (`PrimitiveComponent.SetMaterial` (`self.PR2`) 0 "/Engine/VREditor/BasicMeshes/MI_Cube_03.MI_Cube_03")
    (`PrimitiveComponent.SetMaterial` (`self.PR1`) 0 "/Engine/VREditor/BasicMeshes/MI_Cube_03.MI_Cube_03")
    (clear `PrimitiveComponent.OnClicked` _pr4)
    (clear `PrimitiveComponent.OnClicked` (`self.PR3`))
    (clear `PrimitiveComponent.OnClicked` (`self.PR2`))
    (clear `PrimitiveComponent.OnClicked` (`self.PR1`))
    (else
      (`PrimitiveComponent.SetMaterial` (`self.PR4`) 0 "/Engine/MapTemplates/Sky/M_BlackBackground.M_BlackBackground")
      (`PrimitiveComponent.SetMaterial` (`self.PR3`) 0 "/Engine/MapTemplates/Sky/M_BlackBackground.M_BlackBackground")
      (`PrimitiveComponent.SetMaterial` (`self.PR2`) 0 "/Engine/MapTemplates/Sky/M_BlackBackground.M_BlackBackground")
      (`PrimitiveComponent.SetMaterial` (`self.PR1`) 0 "/Engine/MapTemplates/Sky/M_BlackBackground.M_BlackBackground")
      (add `PrimitiveComponent.OnClicked` (`self.PR1`) (`|CreateDelegate` :!event `Move Pawn`))
      (add `PrimitiveComponent.OnClicked` (`self.PR2`) (`|CreateDelegate` :!event `Move Pawn`))
      (add `PrimitiveComponent.OnClicked` (`self.PR3`) (`|CreateDelegate` :!event `Move Pawn`))
      (add `PrimitiveComponent.OnClicked` (`self.PR4`) (`|CreateDelegate` :!event `Move Pawn`)))))

(fn `HighlightAndMakeMovableYellow`
  (params (IsUnhighlight :type Boolean))
  (bind _py1 (`self.PY1`))
  (bind _py1_2 (`self.PY1`))
  (if IsUnhighlight
    (`PrimitiveComponent.SetMaterial` _py1_2 0 "/Engine/VREditor/BasicMeshes/MI_Cube_01.MI_Cube_01")
    (`PrimitiveComponent.SetMaterial` (`self.PY4`) 0 "/Engine/VREditor/BasicMeshes/MI_Cube_01.MI_Cube_01")
    (`PrimitiveComponent.SetMaterial` (`self.PY3`) 0 "/Engine/VREditor/BasicMeshes/MI_Cube_01.MI_Cube_01")
    (`PrimitiveComponent.SetMaterial` (`self.PY2`) 0 "/Engine/VREditor/BasicMeshes/MI_Cube_01.MI_Cube_01")
    (clear `PrimitiveComponent.OnClicked` _py1_2)
    (clear `PrimitiveComponent.OnClicked` (`self.PY4`))
    (clear `PrimitiveComponent.OnClicked` (`self.PY3`))
    (clear `PrimitiveComponent.OnClicked` (`self.PY2`))
    (else
      (`PrimitiveComponent.SetMaterial` _py1 0 "/Engine/MapTemplates/Sky/M_BlackBackground.M_BlackBackground")
      (`PrimitiveComponent.SetMaterial` (`self.PY4`) 0 "/Engine/MapTemplates/Sky/M_BlackBackground.M_BlackBackground")
      (`PrimitiveComponent.SetMaterial` (`self.PY3`) 0 "/Engine/MapTemplates/Sky/M_BlackBackground.M_BlackBackground")
      (`PrimitiveComponent.SetMaterial` (`self.PY2`) 0 "/Engine/MapTemplates/Sky/M_BlackBackground.M_BlackBackground")
      (add `PrimitiveComponent.OnClicked` _py1 (`|CreateDelegate` :!event `Move Pawn`))
      (add `PrimitiveComponent.OnClicked` (`self.PY4`) (`|CreateDelegate` :!event `Move Pawn`))
      (add `PrimitiveComponent.OnClicked` (`self.PY3`) (`|CreateDelegate` :!event `Move Pawn`))
      (add `PrimitiveComponent.OnClicked` (`self.PY2`) (`|CreateDelegate` :!event `Move Pawn`)))))

(fn `HighlightSelectedPlayerAndMakeItMovable`
  (switch `int` (`KismetMathLibrary.Conv_ByteToInt` (`self.PlayerTurn`))
    (:`0`
      (`self.HighlightAndMakeMovableRed` false))
    (:`1`
      (`self.HighlightAndMakeMovableGreen` false))
    (:`2`
      (`self.HighlightAndMakeMovableBlue` false))
    (:`3`
      (`self.HighlightAndMakeMovableYellow` false))))

(fn `SelectNextPlayer`
  (switch `/Game/RollAndKill/Blueprints/BoardLevel/Enums/PlayerTurnEnum` (`self.PlayerTurn`)
    (:`NewEnumerator0`
      (set `self.PlayerTurn` "NewEnumerator1"))
    (:`NewEnumerator1`
      (set `self.PlayerTurn` "NewEnumerator2"))
    (:`NewEnumerator2`
      (set `self.PlayerTurn` "NewEnumerator3"))
    (:`NewEnumerator3`
      (set `self.PlayerTurn` "NewEnumerator0"))))

(fn `SetDiceLocationBasedOnThePlayerEnum`
  (`SceneComponent.K2_SetRelativeLocation` (`self.Dice`) (`|GetArrayItem` (`self.PlayerTurnDiceLocations`) (`KismetMathLibrary.Conv_ByteToInt` (`self.PlayerTurn`))) false false)
  (bind _returnvalue (`GameplayStatics.GetActorOfClass` "/Game/RollAndKill/Blueprints/BoardLevel/BP_Dice.BP_Dice_C"))
  (`/Engine/EditorBlueprintResources/StandardMacros.IsValid` _returnvalue
    (:`Is Valid`
      (bind _output_get (set `self.DiceRef` _returnvalue))
      (add `/Game/RollAndKill/Blueprints/BoardLevel/BP_Dice.OnDiceRoll` _output_get (`|CreateDelegate` :!event `HighlightSelectedPlayerAndMakeItMovable`)))))

(fn `UserConstructionScript`)