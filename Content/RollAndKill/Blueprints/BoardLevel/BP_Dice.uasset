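; Clickable board-game dice actor that plays a tumble animation, rolls a random number and announces it through an OnDiceRoll call.
; A click passes a DoOnce gate, reopened by RotaionComplete, and starts a timeline that lerps toward randomly picked rotations.
; Each update also rerolls the number and toggles pip visibility to show one, two, three, four or eight.
; On finish it restores the starting rotation, keeping the last roll.
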(event `self.ReceiveBeginPlay`
  (add `self.OnClicked` (delegate `DiceClickEvent`))
  (bind _returnvalue (`GameplayStatics.GetActorOfClass` "/Game/RollAndKill/Blueprints/BoardLevel/BP_Board.BP_Board_C"))
  (set `self.SquareBoardRef` _returnvalue))

(event `DiceClickEvent` :!signature `self.OnClicked`
  (params (TouchedActor :type "Actor Object Reference") (ButtonPressed :type "Key Structure" :default "None"))
  (`/Engine/EditorBlueprintResources/StandardMacros.DoOnce` false :!label _label
    (:`Completed`
      (`self.Rotate Dice`))))

(event `RotaionComplete`
  (goto _label :!via `Reset`))

(event `Rotate Dice`
  (bind (_returnvalue_location _returnvalue_rotation) (`KismetMathLibrary.BreakTransform` (`SceneComponent.GetRelativeTransform` (`self.Dice`))))
  (set `self.DiceCurrentRotaion` _returnvalue_rotation)
  (bind (_direction _newtrack_1) (`Timeline|Timeline` :!via `PlayFromStart`)
    (:`Update`
      (`SceneComponent.K2_SetRelativeRotation` (`self.Dice`) (`KismetMathLibrary.RLerp` (`self.DiceCurrentRotaion`) (`KismetArrayLibrary.Array_Random` (`self.RandomRotations`)) _newtrack_1) false false)
      (`self.Generate Random Dice Number`))
    (:`Finished`
      (`SceneComponent.K2_SetRelativeRotation` (`self.Dice`) (`self.DiceCurrentRotaion`) false false)
      (`self.OnDiceRoll`)
      (`KismetSystemLibrary.PrintString` (`KismetStringLibrary.Conv_IntToString` (`self.RandomDiceSelectedNumber`))))))

(event `Generate Random Dice Number`
  (`self.SetPointsVisibilityBasedOnTheRandomDiceNumber` (`self.GenerateRandomNumberForDice`)))

(fn `GenerateRandomNumberForDice`
  (returns (RandomNumber :type Integer))
  (bind _output_get (set `self.RandomDiceSelectedNumber` (`KismetArrayLibrary.Array_Random` (`self.RandomDiceNumbers`))))
  (return _output_get))

(fn `SetDicePointsForEight`
  (`SceneComponent.SetVisibility` (`self.Points3`) false false)
  (`SceneComponent.SetVisibility` (`self.Points1`) true false)
  (`SceneComponent.SetVisibility` (`self.Points`) true false)
  (`SceneComponent.SetVisibility` (`self.Points8`) true false)
  (`SceneComponent.SetVisibility` (`self.Points7`) true false)
  (`SceneComponent.SetVisibility` (`self.Points4`) true false)
  (`SceneComponent.SetVisibility` (`self.Points6`) true false)
  (`SceneComponent.SetVisibility` (`self.Points5`) true false)
  (`SceneComponent.SetVisibility` (`self.Points2`) true false))

(fn `SetDicePointsForFour`
  (`SceneComponent.SetVisibility` (`self.Points2`) false false)
  (`SceneComponent.SetVisibility` (`self.Points`) false false)
  (`SceneComponent.SetVisibility` (`self.Points7`) false false)
  (`SceneComponent.SetVisibility` (`self.Points6`) false false)
  (`SceneComponent.SetVisibility` (`self.Points3`) false false)
  (`SceneComponent.SetVisibility` (`self.Points8`) true false)
  (`SceneComponent.SetVisibility` (`self.Points4`) true false)
  (`SceneComponent.SetVisibility` (`self.Points5`) true false)
  (`SceneComponent.SetVisibility` (`self.Points1`) true false))

(fn `SetDicePointsForOne`
  (`SceneComponent.SetVisibility` (`self.Points1`) false false)
  (`SceneComponent.SetVisibility` (`self.Points`) false false)
  (`SceneComponent.SetVisibility` (`self.Points8`) false false)
  (`SceneComponent.SetVisibility` (`self.Points7`) false false)
  (`SceneComponent.SetVisibility` (`self.Points4`) false false)
  (`SceneComponent.SetVisibility` (`self.Points6`) false false)
  (`SceneComponent.SetVisibility` (`self.Points5`) false false)
  (`SceneComponent.SetVisibility` (`self.Points2`) false false)
  (`SceneComponent.SetVisibility` (`self.Points3`) true false))

(fn `SetDicePointsForThree`
  (`SceneComponent.SetVisibility` (`self.Points4`) true false)
  (`SceneComponent.SetVisibility` (`self.Points5`) true false)
  (`SceneComponent.SetVisibility` (`self.Points3`) true false)
  (`SceneComponent.SetVisibility` (`self.Points1`) false false)
  (`SceneComponent.SetVisibility` (`self.Points`) false false)
  (`SceneComponent.SetVisibility` (`self.Points8`) false false)
  (`SceneComponent.SetVisibility` (`self.Points7`) false false)
  (`SceneComponent.SetVisibility` (`self.Points6`) false false)
  (`SceneComponent.SetVisibility` (`self.Points2`) false false))

(fn `SetDicePointsForTwo`
  (`SceneComponent.SetVisibility` (`self.Points2`) false false)
  (`SceneComponent.SetVisibility` (`self.Points1`) false false)
  (`SceneComponent.SetVisibility` (`self.Points`) false false)
  (`SceneComponent.SetVisibility` (`self.Points8`) false false)
  (`SceneComponent.SetVisibility` (`self.Points7`) false false)
  (`SceneComponent.SetVisibility` (`self.Points6`) false false)
  (`SceneComponent.SetVisibility` (`self.Points3`) false false)
  (`SceneComponent.SetVisibility` (`self.Points5`) true false)
  (`SceneComponent.SetVisibility` (`self.Points4`) true false))

(fn `SetPointsVisibilityBasedOnTheRandomDiceNumber`
  (params (RandomDiceNumber :type Integer))
  (switch `int` RandomDiceNumber
    (:`Default`
      (`self.SetDicePointsForEight`))
    (:`1`
      (`self.SetDicePointsForOne`))
    (:`2`
      (`self.SetDicePointsForTwo`))
    (:`3`
      (`self.SetDicePointsForThree`))
    (:`4`
      (`self.SetDicePointsForFour`))))

(fn `UserConstructionScript`)